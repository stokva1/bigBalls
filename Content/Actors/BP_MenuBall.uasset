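; BP_MenuBall is a ball actor, apparently for the menu, that displays the player's selected skin.
; On BeginPlay it reads SkinID from BP_GameInstance and applies the matching SkinArray material to its static mesh.
; ChangeTextureLeft looks like a placeholder: it prints a debug string and sets a hardcoded M_Bush material instead of stepping through the skin array.
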(event EventBeginPlay
  (bind _asbp_game_instance (Utilities|Casting|CastToBP_GameInstance (Game|GetGameInstance)))
  (Rendering|Material|SetMaterial (Variables|Default|GetStaticMesh) 0 (Utilities|Array|Get(acopy) (Variables|/Game/BP_GameInstance.BP_GameInstance_C|GetSkinArray _asbp_game_instance) (Variables|/Game/BP_GameInstance.BP_GameInstance_C|GetSkin_ID _asbp_game_instance))))

(event Collision|EventActorBeginOverlap
  (params (OtherActor :type Actor%20Object%20Reference)))

(event EventTick
  (params (DeltaSeconds :type Float%20%28single-precision%29)))

(fn ConstructionScript)

(fn ChangeTextureLeft
  (Development|PrintString "Hello")
  (Rendering|Material|SetMaterial (Variables|Default|GetStaticMesh) 0 "/Game/StarterContent/Props/Materials/M_Bush.M_Bush"))