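; BP_HC is a heart pickup actor that grants one health when a BP_Ball overlaps it.
; On overlap it passes itself to MapLevelAddOneHealth on BP_GameInstance and plays the Heart_pickup sound in 2D.
; Tick spins the heart around its local yaw axis at a rate set by Rotation, scaled by delta time.
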(event EventBeginPlay)

(event Collision|EventActorBeginOverlap
  (params (OtherActor :type Actor%20Object%20Reference))
  (bind _asbp_game_instance (Utilities|Casting|CastToBP_GameInstance (Game|GetGameInstance)))
  (Utilities|Casting|CastToBP_Ball OtherActor)
  (Default|MapLevelAddOneHealth _asbp_game_instance self)
  (Audio|PlaySound2D "/Game/Sounds/heart_pickup.heart_pickup" 1.0 1.0 0.0 0 0))

(event EventTick
  (params (DeltaSeconds :type Float%20%28single-precision%29))
  ;[1 1 1] Rotate heart
  (Transformation|AddActorLocalRotation (Math|Rotator|MakeRotator 0.0 0.0 (* DeltaSeconds (Variables|Default|GetRotation))) false false))

(fn ConstructionScript)