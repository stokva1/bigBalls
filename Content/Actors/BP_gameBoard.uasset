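; Game board actor that the player tilts with WASD, up to a limit on each axis.
; Key events set held flags, and Tick steps roll (W/S) and pitch (A/D) by a fixed per-frame speed, applying the rotation without physics teleport.
; Escape creates WB_PauseMenu and pauses the game, but immediately resets its open flag, so its close-and-unpause branch is never reached.
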(event EventBeginPlay
  (Input|EnableInput (Game|GetPlayerController 0)))

(event Collision|EventActorBeginOverlap
  (params (OtherActor :type Actor%20Object%20Reference)))

(event EventTick
  (params (DeltaSeconds :type Float%20%28single-precision%29))
  (Transformation|SetActorRotation (Math|Rotator|MakeRotator (Variables|Default|GetTiltAngleX) (Variables|Default|GetTiltAngleY) 0.0))
  (Utilities|FlowControl|Sequence
    (:then_0
      (if (Variables|Default|GetW_held)
        (if (< (+ (Variables|Default|GetTiltAngleX) (Variables|Default|GetTiltSpeed)) (Variables|Default|GetMaxTiltAngel))
          (Variables|Default|SetTiltAngleX (+ (Variables|Default|GetTiltAngleX) (Variables|Default|GetTiltSpeed))))
        (elif (Variables|Default|GetS_held)
          (if (> (- (Variables|Default|GetTiltAngleX) (Variables|Default|GetTiltSpeed)) (* (Variables|Default|GetMaxTiltAngel) -1.0))
            (Variables|Default|SetTiltAngleX (- (Variables|Default|GetTiltAngleX) (Variables|Default|GetTiltSpeed)))))))
    (:then_1
      (if (Variables|Default|GetD_held)
        (if (< (+ (Variables|Default|GetTiltAngleY) (Variables|Default|GetTiltSpeed)) (Variables|Default|GetMaxTiltAngel))
          (Variables|Default|SetTiltAngleY (+ (Variables|Default|GetTiltAngleY) (Variables|Default|GetTiltSpeed))))
        (elif (Variables|Default|GetA_held)
          (if (> (- (Variables|Default|GetTiltAngleY) (Variables|Default|GetTiltSpeed)) (* (Variables|Default|GetMaxTiltAngel) -1.0))
            (Variables|Default|SetTiltAngleY (- (Variables|Default|GetTiltAngleY) (Variables|Default|GetTiltSpeed)))))))))

(event Input|KeyboardEvents|Escape
  (params (Key :type Key%20Structure :default "None"))
  ;[0.15 0.15 0.15 0.5] Handle open resume menu
  (:Pressed
    (if (not (Variables|Default|GetisPauseMenuOpened))
      (Variables|Default|SetisPauseMenuOpened true)
      (bind _returnvalue (UserInterface|CreateWidget "/Game/UI/WB_PauseMenu.WB_PauseMenu_C" (Game|GetPlayerController 0)))
      (bind _output_get (Variables|Default|SetPause%20menu%20widget _returnvalue))
      (UserInterface|Viewport|AddtoViewport _output_get 0)
      (Game|SetGamePaused true)
      (Variables|Default|SetisPauseMenuOpened false)
      (else
        (Variables|Default|SetisPauseMenuOpened false)
        (Widget|RemovefromParent (Variables|Default|GetPause%20menu%20widget))
        (Game|SetGamePaused false)))))

(event Input|KeyboardEvents|D
  (params (Key :type Key%20Structure :default "None"))
  (:Pressed
    (Variables|Default|SetD_held true))
  (:Released
    (Variables|Default|SetD_held false)))

(event Input|KeyboardEvents|W
  (params (Key :type Key%20Structure :default "None"))
  (:Pressed
    (Variables|Default|SetW_held true))
  (:Released
    (Variables|Default|SetW_held false)))

(event Input|KeyboardEvents|S
  (params (Key :type Key%20Structure :default "None"))
  (:Pressed
    (Variables|Default|SetS_held true))
  (:Released
    (Variables|Default|SetS_held false)))

(event Input|KeyboardEvents|A
  (params (Key :type Key%20Structure :default "None"))
  (:Pressed
    (Variables|Default|SetA_held true))
  (:Released
    (Variables|Default|SetA_held false)))

(fn ConstructionScript)